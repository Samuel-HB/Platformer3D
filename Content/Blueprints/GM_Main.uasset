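; GM_Main is the main game mode Blueprint, managing a checkpoint and respawn position for the player.
; On BeginPlay it seeds the checkpoint from the player controller's location and binds to checkpoint-reached and player-death event dispatchers.
; SetNewCheckPoint stores the character's current location, and SetPlayerPosition moves the character back to the stored checkpoint.
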(event `self.ReceiveBeginPlay`
  (set `self.checkPoint` (`self.K2_GetActorLocation` (`GameplayStatics.GetPlayerController` 0)))
  (add `self.PlayerReachingCheckPointEventDispatcher` (`|CreateDelegate` :!event `SetNewCheckPoint`))
  (add `self.OnPlayerDeathEventDispatcher` (`|CreateDelegate` :!event `SetPlayerPosition`)))

(fn `SetNewCheckPoint`
  (set `self.checkPoint` (`self.K2_GetActorLocation` (`GameplayStatics.GetPlayerCharacter` 0))))

(fn `SetPlayerPosition`
  (`self.K2_SetActorLocation` (`GameplayStatics.GetPlayerCharacter` 0) (`self.checkPoint`) false false))

(fn `UserConstructionScript`)