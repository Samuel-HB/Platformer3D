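; BP_BoostCollectible is a respawning pickup that calls SetWallRunState on the player when overlapped.
; Its collision sphere reacts only to BP_Player, then deactivates the pickup by hiding the mesh, disabling collision and stopping the root component's tick.
; A short timer then reverses those changes, so the same actor is reused instead of destroyed.
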(event `self.SphereCollision.OnComponentBeginOverlap`
  (params (OverlappedComponent :type "PrimitiveComponent Object Reference") (OtherActor :type "Actor Object Reference") (OtherComp :type "PrimitiveComponent Object Reference") (OtherBodyIndex :type Integer) (bFromSweep :type Boolean) (SweepResult :type "HitResult Structure (by ref)"))
  (bind _asbp_player (cast `/Game/Blueprints/BP_Player` OtherActor))
  (`/Game/Blueprints/BP_Player.SetWallRunState` _asbp_player)
  (`self.DeactivateCollectible`))

(event `DeactivateCollectible`
  (`SceneComponent.SetVisibility` (`self.Sphere`) false true)
  (`PrimitiveComponent.SetCollisionEnabled` (`self.SphereCollision`) "NoCollision")
  (`ActorComponent.SetComponentTickEnabled` (`self.DefaultSceneRoot`) false)
  (`KismetSystemLibrary.K2_SetTimerDelegate` (delegate `ActivateCollectible`) 1.5))

(event `ActivateCollectible`
  (`SceneComponent.SetVisibility` (`self.Sphere`) true true)
  (`PrimitiveComponent.SetCollisionEnabled` (`self.SphereCollision`) "QueryAndPhysics")
  (`ActorComponent.SetComponentTickEnabled` (`self.DefaultSceneRoot`) true))

(fn `UserConstructionScript`)